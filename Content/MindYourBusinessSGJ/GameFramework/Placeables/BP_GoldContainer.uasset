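; BP_GoldContainer is a damageable placeable that displays the player's gold and triggers the lose screen when its health runs out.
; Every tick it scales IncreasingGoldMesh uniformly by mapping the game mode's current gold against its maximum.
; ApplyDamage lowers clamped Health and, at zero, finds the main UI widget to create the lose widget.
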(event `self.ReceiveTick`
  (params (DeltaSeconds :type "Float (single-precision)"))
  (bind _asgm_mine_your_business (cast `/Game/MindYourBusinessSGJ/GameFramework/GM_MineYourBusiness` (`GameplayStatics.GetGameMode`)))
  (bind _returnvalue (`KismetMathLibrary.MapRangeClamped` (`/Game/MindYourBusinessSGJ/GameFramework/GM_MineYourBusiness.CurrentGold` _asgm_mine_your_business) 0.0 (`/Game/MindYourBusinessSGJ/GameFramework/GM_MineYourBusiness.MaximumGold` _asgm_mine_your_business) 0.0 1.5))
  (`SceneComponent.SetWorldScale3D` (`self.IncreasingGoldMesh`) (`KismetMathLibrary.MakeVector` _returnvalue _returnvalue _returnvalue)))

(event `ApplyDamage`
  (params (DamageToApply :type "Float (double-precision)"))
  (bind _output_get (set `self.Health` (`KismetMathLibrary.FClamp` (- (`self.Health`) DamageToApply) 0.0 100.0)))
  (if (<= _output_get 0.0)
    (bind _foundwidgets (`WidgetBlueprintLibrary.GetAllWidgetsOfClass` "/Game/MindYourBusinessSGJ/UI/Gameplay/WBP_MainUI.WBP_MainUI_C"))
    (`/Game/MindYourBusinessSGJ/UI/Gameplay/WBP_MainUI.CreateWinLoseWidget` (`|GetArrayItem` _foundwidgets) false)))

(fn `UserConstructionScript`)