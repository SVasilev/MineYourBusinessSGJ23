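; BP_Robot_Fixer is a robot character that walks to a gold container and repairs it.
; On BeginPlay it uses AIMoveTo to reach the target's FixPoint, snaps to a fixed rotation and spawns a spark emitter ahead of itself.
; A looping timer then drives FixContainer, where a timeline animates the body mesh along X, then applies negative damage as healing and plays a welding sound.
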(event `FixContainer`
  (bind _bodymesh (`self.BodyMesh`))
  (bind (_relativelocation_x _relativelocation_y _relativelocation_z) (`KismetMathLibrary.BreakVector` (`SceneComponent.RelativeLocation` _bodymesh)))
  (bind (_direction _newtrack_0) (`Timeline|Timeline` :!via `PlayFromStart`)
    (:`Update`
      (`SceneComponent.K2_SetRelativeLocation` _bodymesh (`KismetMathLibrary.MakeVector` _newtrack_0 _relativelocation_y _relativelocation_z) false true))
    (:`Finished`
      (`/Game/MindYourBusinessSGJ/GameFramework/Placeables/BP_GoldContainer.ApplyDamage` (`self.GoldContainerTarget`) -5.0)
      (`GameplayStatics.PlaySound2D` "/Game/MindYourBusinessSGJ/Audio/SFX/Welding.Welding" 1.0 1.0 0.0 null null))))

(event `self.ReceiveBeginPlay`
  (`parent.ReceiveBeginPlay`)
  (`|AIMoveTo` self (`SceneComponent.K2_GetComponentLocation` (`/Game/MindYourBusinessSGJ/GameFramework/Placeables/BP_GoldContainer.FixPoint` (`self.GoldContainerTarget`))) null
    (:`OnSuccess`
      (`self.K2_SetActorRotation` (struct :`Yaw` -135.0))
      (`|ExecutionSequence`
        (:`then_0`
          (`GameplayStatics.SpawnEmitterAtLocation` "/Game/VFX_Toolkit_V1/ParticleSystems/356Days/Par_SparCore_01.Par_SparCore_01" (+ (`self.K2_GetActorLocation`) (* (`self.GetActorForwardVector`) (150.0 150.0 150.0))) (struct) (1.0 1.0 1.0) false))
        (:`then_1`
          (`KismetSystemLibrary.K2_SetTimerDelegate` (delegate `FixContainer`) 1.5 true)
          (`self.FixContainer`))))))

(fn `UserConstructionScript`
  (`parent.UserConstructionScript`))