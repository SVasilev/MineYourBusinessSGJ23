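; BP_Robot_Annihilator is a robot that hunts a sentient miner and destroys it in an explosion.
; On BeginPlay it looks for the first BP_Robot_Miner flagged IsSentient, using a looping timer when none is found.
; Once one is found, it clears the timer and uses AI MoveTo to approach.
; On arrival it spawns explosion particles and destroys all Pawn-type actors in a sphere around itself, with no ignore list.
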(event `self.ReceiveBeginPlay`
  (`parent.ReceiveBeginPlay`)
  (`self.TryDestroySentientMiner`))

(event `TryDestroySentientMiner`
  (bind _returnvalue (`self.K2_GetActorLocation`))
  (bind _result (`self.FindSentientMiner`))
  (`/Engine/EditorBlueprintResources/StandardMacros.IsValid` _result
    (:`Is Valid`
      (`KismetSystemLibrary.K2_ClearAndInvalidateTimerHandle` (`self.NewVar`))
      (`|AIMoveTo` self (0.0 0.0 0.0) _result
        (:`OnSuccess`
          (`GameplayStatics.SpawnEmitterAtLocation` "/Game/VFX_Toolkit_V1/ParticleSystems/356Days/Par_BombWaker.Par_BombWaker" _returnvalue (struct) (0.75 0.75 0.75))
          (`GameplayStatics.SpawnEmitterAtLocation` "/Game/VFX_Toolkit_V1/ParticleSystems/356Days/Par_ToonBoom2.Par_ToonBoom2" _returnvalue (struct) (0.75 0.75 0.75))
          (bind _outactors (`KismetSystemLibrary.SphereOverlapActors` _returnvalue 200.0 (`|MakeArray` "ObjectTypeQuery3" :!type "EObjectTypeQuery Enum")))
          (for _array_element _outactors
            (`self.K2_DestroyActor` _array_element)))))
    (:`Is Not Valid`
      (bind _returnvalue_2 (`KismetSystemLibrary.K2_SetTimerDelegate` (`|CreateDelegate` :!event `TryDestroySentientMiner`) 1.0 true))
      (set `self.NewVar` _returnvalue_2))))

(fn `FindSentientMiner`
  (returns (Result :type "/Game/MindYourBusinessSGJ/GameFramework/Characters/Robot/BP_Robot_Miner Object Reference"))
  (bind _outactors (`GameplayStatics.GetAllActorsOfClass` "/Game/MindYourBusinessSGJ/GameFramework/Characters/Robot/BP_Robot_Miner.BP_Robot_Miner_C"))
  (for _array_element _outactors
    (if (`/Game/MindYourBusinessSGJ/GameFramework/Characters/Robot/BP_Robot_Miner.bIsSentient` _array_element)
      (return _array_element))))

(fn `UserConstructionScript`
  (`parent.UserConstructionScript`))